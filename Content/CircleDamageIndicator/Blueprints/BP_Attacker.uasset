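; BP_Attacker is a test enemy in the CircleDamageIndicator project that turns to face player pawn 0 every Tick and damages it when Fire is triggered.
; Attack line-traces on Visibility and, on hitting BP_FirstPersonCharacter, lowers its Health directly and applies point damage carrying the attacker-to-player direction.
; An explosion emitter then spawns at the attacker's location.
; The timer for automatic repeat attacks is disconnected.
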(event `Fire`
  (`self.Attack`))

(event `self.ReceiveBeginPlay`)

(event `self.ReceiveTick`
  (params (DeltaSeconds :type "Float (single-precision)"))
  (bind _returnvalue (`GameplayStatics.GetPlayerPawn` 0))
  ;[1 1 1] Look at player
  (if (`KismetSystemLibrary.IsValid` _returnvalue)
    (`self.K2_SetActorRotation` (`KismetMathLibrary.FindLookAtRotation` (`self.K2_GetActorLocation`) (`self.K2_GetActorLocation` _returnvalue)))
    (else
      (`KismetSystemLibrary.PrintString` "Player pawn not found" true true (struct :`R` 1.0 :`A` 1.0) 0.0))))

(fn `Attack`
  (bind _returnvalue (`GameplayStatics.GetPlayerPawn` 0))
  (bind _returnvalue_2 (`self.K2_GetActorLocation`))
  (bind _returnvalue_3 (`self.K2_GetActorLocation` _returnvalue))
  (if (`KismetSystemLibrary.IsValid` _returnvalue)
    ;[1 1 1] Check player visibility
    (bind _outhit (`KismetSystemLibrary.LineTraceSingle` :`Start` _returnvalue_2 :`End` _returnvalue_3 :`TraceChannel` "TraceTypeQuery1" :`DrawTime` 0.5)) ; Player is visible?
    (bind _asbp_first_person_character (cast `/Game/FirstPerson/Blueprints/BP_FirstPersonCharacter` (`.HitActor` (`GameplayStatics.BreakHitResult` _outhit)))
      (:`then`
        ;[1 1 1] Apply damage to player and create explosion
        (set `/Game/FirstPerson/Blueprints/BP_FirstPersonCharacter.Health` (- (`/Game/FirstPerson/Blueprints/BP_FirstPersonCharacter.Health` _asbp_first_person_character) 10.0) _asbp_first_person_character)
        (`GameplayStatics.ApplyPointDamage` _asbp_first_person_character 1.0 (`KismetMathLibrary.GetDirectionUnitVector` _returnvalue_2 _returnvalue_3) _outhit null self "/Script/Engine.DamageType") ; Damage him
        (`GameplayStatics.SpawnEmitterAtLocation` "/Game/CircleDamageIndicator/Particles/P_Explosion.P_Explosion" (`self.K2_GetActorLocation`)) ; And spawn explode particle
      )
      (:`CastFailed`
        (`KismetSystemLibrary.PrintString` "Attacked actor is not player" false true (struct :`R` 0.9 :`G` 0.417156 :`A` 1.0) 0.5)))
    (else
      (`KismetSystemLibrary.PrintString` "Player pawn not found" true true (struct :`R` 1.0 :`G` 0.106649 :`A` 1.0) 0.0))))

(fn `UserConstructionScript`)