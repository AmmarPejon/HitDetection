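; HitDetector turns incoming damage into directional bHaptics feedback for its owning actor.
; DamageTaken measures the distance and signed horizontal angle from the owner's facing to the hit source, wrapped into ±180 degrees, and prints both.
; If bHaptics is available, HapticEvents maps the angle to front, side or back zone patterns, randomly choosing upper or lower variants toward the front.
; Distance does not affect which haptic plays.
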(fn `Damage Taken`
  (params (`From Location` :type "Vector Structure"))
  (`self.Init`)
  (`self.Measure Distance` `From Location`)
  (`self.Measure Angle` `From Location`)
  (`self.Print Data`)
  (bind _returnvalue (`BhapticsSDK2.IsBhapticsAvailable`))
  (if _returnvalue
    (`self.HapticEvents`)
    (else
      (`KismetSystemLibrary.PrintString` "bHaptics environment not set up"))))

(fn `HapticEvents`
  (bind _angle (`self.Angle`))
  (bind _angle_2 (`self.Angle`))
  (bind _angle_3 (`self.Angle`))
  (if (>= _angle -20.0)
    (if (<= _angle 20.0)
      ;[1 1 1] Center
      (if (`KismetMathLibrary.RandomBool`)
        (`BhapticsSDK2.PlayHaptic` "higher_center_damage")
        (else
          (`BhapticsSDK2.PlayHaptic` "lower_center_damage")))
      (elif (<= _angle_2 80.0)
        ;[1 1 1] Right Side
        (if (`KismetMathLibrary.RandomBool`)
          (`BhapticsSDK2.PlayHaptic` "lower_right_damage")
          (else
            (`BhapticsSDK2.PlayHaptic` "upper_right_damage")))
        (elif (<= _angle_2 120.0)
          (`BhapticsSDK2.PlayHaptic` "right_damage")
          (elif (<= _angle_2 160.0)
            (`BhapticsSDK2.PlayHaptic` "back_right_damage")
            (else
              (`BhapticsSDK2.PlayHaptic` "back_center_damage"))))))
    (elif (>= _angle_3 -80.0)
      ;[1 1 1] Left Side
      (if (`KismetMathLibrary.RandomBool`)
        (`BhapticsSDK2.PlayHaptic` "lower_left_damage")
        (else
          (`BhapticsSDK2.PlayHaptic` "upper_left_damage")))
      (elif (>= _angle_3 -120.0)
        (`BhapticsSDK2.PlayHaptic` "left_damage")
        (elif (>= _angle_3 -160.0)
          (`BhapticsSDK2.PlayHaptic` "back_left_damage")
          (else
            (`BhapticsSDK2.PlayHaptic` "back_center_damage")))))))

(fn `Init`
  (set `self.Distance` 0.0)
  (set `self.Angle` 0.0))

(fn `Measure Angle`
  (params (`From Location` :type "Vector Structure"))
  (bind _returnvalue (`self.GetOwner`))
  (bind _returnvalue_2 (- (.yaw (`KismetMathLibrary.Conv_VectorToRotator` (`KismetMathLibrary.Normal` (* (`KismetMathLibrary.GetDirectionUnitVector` `From Location` (`Actor.K2_GetActorLocation` _returnvalue)) (-1.0 -1.0 0.0))))) (.yaw (`KismetMathLibrary.Conv_VectorToRotator` (`KismetMathLibrary.Normal` (`Actor.GetActorForwardVector` _returnvalue))))))
  (set `self.Angle` _returnvalue_2)
  (if (>= _returnvalue_2 180.0)
    (set `self.Angle` (- (`self.Angle`) 360.0))
    (elif (<= _returnvalue_2 -180.0)
      (set `self.Angle` (+ (`self.Angle`) 360.0)))))

(fn `Measure Distance`
  (params (`From Location` :type "Vector Structure"))
  (set `self.Distance` (`KismetMathLibrary.VSize` (- (`Actor.K2_GetActorLocation` (`self.GetOwner`)) `From Location`))))

(fn `Print Data`
  (`KismetSystemLibrary.PrintString` (`KismetStringLibrary.Concat_StrStr` "Distance: " (`KismetStringLibrary.Conv_DoubleToString` (`self.Distance`))))
  (`KismetSystemLibrary.PrintString` (`KismetStringLibrary.Concat_StrStr` "Angle: " (`KismetStringLibrary.Conv_DoubleToString` (`self.Angle`)))))